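; ItemWorldActor is a world actor that represents an item, with a 3D mesh and a floating name label.
; On BeginPlay it reads the class defaults of its ItemSignature to set the static mesh and fill the name text in its WorldActorWB widget.
; Every tick it shows the widget only while the player character is within a set distance, rotating it to face that character's follow camera.
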(event EventBeginPlay
  (CallFunction|Initialize3dMesh)
  (CallFunction|InitializeWidget))

(event EventTick
  (params (DeltaSeconds :type Float%20%28single-precision%29))
  (CallFunction|UpdateWidgetRotation))

(fn ConstructionScript)

(fn Initialize3dMesh
  ;[1 1 1] Set Mesh
  (Components|StaticMesh|SetStaticMesh (Variables|Default|GetStaticMesh) (.mesh (Utilities|GetClassDefaults (Variables|Default|GetItemSignature)))))

(fn InitializeWidget
  ;[1 1 1] Set text in Widget
  (Rendering|Components|TextRender|SetText (Variables|/Game/Widgets/Items/WorldActorWB.WorldActorWB_C|GetItemName_TextBox (.AsWorld%20Actor%20WB (Utilities|Casting|CastToWorldActorWB (UserInterface|GetUserWidgetObject (Variables|Default|GetWidget))))) (.name (Utilities|GetClassDefaults (Variables|Default|GetItemSignature)))))

(fn UpdateWidgetRotation
  (bind _widget (Variables|Default|GetWidget))
  (bind _returnvalue (UserInterface|GetUserWidgetObject _widget))
  ;[1 1 1] Change Widget Visibility
  ;;[1 1 1] If distanse to character <4500
  (if (< (Transformation|GetDistanceTo (Game|GetPlayerCharacter 0)) 4.5e+03)
    ;;[1 1 1] Make visible
    (Widget|SetVisibility _returnvalue "Visible")
    ;[1 1 1] Change Widget Rotation
    ;;[1 1 1] Rotate Widget to Camera
    (Transformation|SetWorldRotation (Variables|Default|GetWidget) (Math|Rotator|FindLookatRotation (Transformation|GetWorldLocation (Variables|Default|GetWidget)) (Transformation|GetWorldLocation (Variables|/Script/SurvivalGame.PlayerCharacter|GetFollowCamera (.AsPlayer%20Character%20BP (Utilities|Casting|CastToPlayerCharacterBP (Game|GetPlayerCharacter 0)))))) false false)
    (else
      ;;[1 1 1] Make Hidden
      (Widget|SetVisibility _returnvalue "Hidden"))))