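; Player character with survival stats, a HUD and F-key item pickup.
; BeginPlay creates MainHUD; Tick drives a one-second Delay that drains hunger, then HP once hunger is empty, refreshing the HUD.
; Reaching zero HP sets the status to Dead and prints a message.
; Pickup line-traces a short distance from the follow camera and destroys any ItemWorldActor hit, without storing it.
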(event EventBeginPlay
  ;[1 1 1] BeginPlay
  ;;[1 1 1] Create and save MainHUD Widget
  (bind _returnvalue (UserInterface|CreateWidget "/Game/Widgets/MainHUD.MainHUD_C"))
  (bind _output_get (Variables|Default|SetMainHUD _returnvalue))
  (UserInterface|Viewport|AddtoViewport _output_get 0)
  ;;[1 1 1] Update HP and Hungry Widget
  (CallFunction|UpdateStatsinHUD))

(event EventTick
  (params (DeltaSeconds :type Float%20%28single-precision%29))
  ;[1 1 1] Event Tick
  (Utilities|LoseHungry))

(event Input|KeyboardEvents|F
  (params (Key :type Key%20Structure :default "None"))
  ;[1 1 1] Pick Up Item by F button
  (:Pressed
    (bind _actor (CallFunction|FindObjectinFrontOfCamera))
    (Utilities|IsValid _actor
      (:Is%20Valid
        (bind _asitem_world_actor (Utilities|Casting|CastToItemWorldActor _actor))
        (Actor|DestroyActor _asitem_world_actor)))))

(fn ConstructionScript)

(fn UpdateStatsinHUD
  (Default|UpdateHPandHungry (Variables|Default|GetMainHUD) (Variables|Health|GetMaxHP) (Variables|Health|GetCurrentHP) (Variables|Health|GetHungry%20Level)))

(fn LoseHP
  (params (Damage :type Float%20%28single-precision%29))
  ;[1 1 1] Reducing HP and checking for death
  ;;[1 1 1] If Player Alive
  (switch Utilities|FlowControl|Switch|SwitchonPlayerStatus (Variables|Default|GetStatus)
    (:NewEnumerator0
      ;;[0 1 0.07145] Reduce HP
      (Variables|Health|SetCurrentHP (- (Variables|Health|GetCurrentHP) Damage))
      ;;[1 1 1] If HP <= 0
      (if (<= (Variables|Health|GetCurrentHP) 0.0)
        (Variables|Health|SetCurrentHP 0.0)
        (CallFunction|Death)))))

(fn FindObjectinFrontOfCamera
  (bind _followcamera (Variables|Default|GetFollowCamera))
  (bind _returnvalue (Transformation|GetWorldLocation _followcamera))
  ;[1 1 1] Line Trace in 300 distance
  (bind _outhit (Collision|LineTraceByChannel _returnvalue (+ _returnvalue (* (Math|Vector|GetForwardVector (Transformation|GetWorldRotation _followcamera)) 3e+02)) "TraceTypeQuery1" false 0 "None"))
  (return (.HitActor (Collision|BreakHitResult _outhit))))

(fn Death
  (Variables|Default|SetStatus "NewEnumerator1")
  (Development|PrintString "Bye bye"))